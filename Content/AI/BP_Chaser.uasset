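; Melee AI enemy character that patrols, detects the player by sight and noise, and carries a baton attached to its hand socket.
; It exposes state such as attack range, cycling patrol targets and last heard noise, registered from BP_Noise capsule overlaps until sight detection completes.
; Tick refreshes player distance and the detection meter widget, or at zero health ragdolls the body, detaches the controller and destroys it after a delay.
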(event `self.ReceiveBeginPlay`
  (bind _mesh (`self.Mesh`))
  ;[1 1 1] Begin Play
  ;;[1 1 1] Set Attack Distance Based on CapsuleRadius
  (set `self.CurrentHealth` (`self.MaxHealth`))
  (bind _ascharacter_bp (cast `/Game/Character/Character_BP` (`Controller.K2_GetPawn` (`GameplayStatics.GetPlayerController` 0)))
    (:`then`
      (set `self.AttackDistance` (+ (`CapsuleComponent.GetScaledCapsuleRadius` (`Character.CapsuleComponent` _ascharacter_bp)) (`CapsuleComponent.GetScaledCapsuleRadius` (`self.CapsuleComponent`)) 5.0))
      ;;[1 1 1] Spawn and Attatch Baton
      (bind _returnvalue (`|SpawnActorFromClass` "/Game/AI/BP_Weapon_baton.BP_Weapon_Baton_C" (`SceneComponent.GetSocketTransform` _mesh "WeaponHolder" "RTS_World") "Undefined" "OverrideRootScale" self null))
      (`self.K2_AttachToComponent` _returnvalue _mesh "WeaponHolder" "SnapToTarget" "SnapToTarget" "SnapToTarget" true)
      (set `self.Baton` _returnvalue)
      (bind _asdetection_hud (cast `/Game/UI/DetectionHUD` (`WidgetComponent.GetUserWidgetObject` (`self.DetectionMeter`))))
      (set `/Game/UI/DetectionHUD.RequiredSenseTime` (`self.RequiredSightTime`) _asdetection_hud))
    (:`CastFailed`
      (`KismetSystemLibrary.PrintString` "Playercontroller not set to character." true true (struct :`R` 1.0 :`B` 0.018495 :`A` 1.0)))))

(event `self.ReceiveTick`
  (params (DeltaSeconds :type "Float (single-precision)"))
  ;[1 1 1] TICK
  ;;[1 1 1] Check health -> Kill
  (if (<= (`self.CurrentHealth`) 0.0)
    (`self.ActorDeath`)
    (else
      ;;[1 1 1] Set Distance to player
      (bind _output_get (set `self.DistanceToPlayer` (`KismetMathLibrary.Abs` (`self.GetDistanceTo` (`GameplayStatics.GetPlayerCharacter` 0)))))
      (set `self.InAttackDistance` (<= _output_get (`self.AttackDistance`)))
      (`self.UpdateDetectionMeter`))))

(event `ActorDeath`
  (bind _mesh (`self.Mesh`))
  ;[1 1 1] Actor Death
  (set `/Game/Character/Weapon_PaintBrush.Active` false (`self.Baton`))
  (`SceneComponent.SetVisibility` (`self.DetectionMeter`) false false)
  (`SkeletalMeshComponent.SetAllBodiesSimulatePhysics` _mesh true)
  (`PrimitiveComponent.SetSimulatePhysics` _mesh true)
  (`PrimitiveComponent.WakeAllRigidBodies` _mesh)
  (`PrimitiveComponent.SetCollisionEnabled` (`self.CapsuleComponent`) "NoCollision")
  (`self.DetachFromControllerPendingDestroy`)
  (`KismetSystemLibrary.Delay` 5.0)
  (`self.K2_DestroyActor` (`self.Baton`))
  (`self.K2_DestroyActor`))

(event `self.CapsuleComponent.OnComponentBeginOverlap`
  (params (OverlappedComponent :type "PrimitiveComponent Object Reference") (OtherActor :type "Actor Object Reference") (OtherComp :type "PrimitiveComponent Object Reference") (OtherBodyIndex :type Integer) (bFromSweep :type Boolean) (SweepResult :type "HitResult Structure (by ref)"))
  (if (and (== (`GameplayStatics.GetObjectClass` OtherActor) "/Game/Blueprints/BP_Noise.BP_Noise_C") (< (`self.ActualSightTime`) (`self.RequiredSightTime`)))
    (set `self.LastNoiseLoc` (`self.K2_GetActorLocation` OtherActor))
    (set `self.HeardNoise` true)))

(fn `GetNextTargetLocation`
  (returns (NextTargetLocation :type "Vector Structure"))
  ;[1 1 1] Check that target array is not empty
  (if (> (`KismetArrayLibrary.Array_Length` (`self.PatrolLocations`)) 0)
    ;[1 1 1] Check if actor at current target
    (if (and (== (`KismetMathLibrary.MakeVector2D` (.x (`self.K2_GetActorLocation` (`|GetArrayItem` (`self.PatrolLocations`) (`self.CurrentTargetIndex`)))) (.y (`self.K2_GetActorLocation` (`|GetArrayItem` (`self.PatrolLocations`) (`self.CurrentTargetIndex`))))) (`KismetMathLibrary.MakeVector2D` (.x (`self.K2_GetActorLocation`)) (.y (`self.K2_GetActorLocation`))) :`ErrorTolerance` 5.0) (`KismetMathLibrary.NearlyEqual_FloatFloat` (.z (`self.K2_GetActorLocation` (`|GetArrayItem` (`self.PatrolLocations`) (`self.CurrentTargetIndex`)))) (.z (`self.K2_GetActorLocation`)) 100.0))
      ;[1 1 1] Return next target if actor at current
      (bind _result (`/Engine/EditorBlueprintResources/StandardMacros.IncrementInt` (`self.CurrentTargetIndex`))
        (:`  `
          (if (not (< _result (`KismetArrayLibrary.Array_Length` (`self.PatrolLocations`))))
            (set `self.CurrentTargetIndex` 0))
          (return (`self.K2_GetActorLocation` (`|GetArrayItem` (`self.PatrolLocations`) (`self.CurrentTargetIndex`))))))
      (else
        ;[1 1 1] Return current target if actor not there
        (return (`self.K2_GetActorLocation` (`|GetArrayItem` (`self.PatrolLocations`) (`self.CurrentTargetIndex`))))))
    (else
      (`KismetSystemLibrary.PrintString` (`KismetStringLibrary.Concat_StrStr` "No Targets for AI: " (`KismetSystemLibrary.GetDisplayName` self)))
      (return (0.0 0.0 0.0)))))

(fn `TakeDamage`
  (set `self.CurrentHealth` (- (`self.CurrentHealth`) 1.0)))

(fn `TakeHeavyDamage`
  (set `self.CurrentHealth` (- (`self.CurrentHealth`) 5.0)))

(fn `UpdateDetectionMeter`
  (bind _asdetection_hud (cast `/Game/UI/DetectionHUD` (`WidgetComponent.GetUserWidgetObject` (`self.DetectionMeter`))))
  (set `/Game/UI/DetectionHUD.ActualSenseTime` (`self.ActualSightTime`) _asdetection_hud))

(fn `UpdateHealthBar`
  (bind _aschaser_health_hud (cast `/Game/UI/ChaserHealthHUD` (`WidgetComponent.GetUserWidgetObject` (`self.DetectionMeter`))))
  (set `/Game/UI/ChaserHealthHUD.HealthPercent` (/ (`self.CurrentHealth`) (`self.MaxHealth`)) _aschaser_health_hud))

(fn `UserConstructionScript`)