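; Baton weapon for the BP_Chaser enemy that kills the player on a hit.
; When its Box begins overlapping the player, it checks that the owning chaser's active montage is a left or right slash within a fixed playback-time window.
; A valid hit calls EventPlayerDeath on Character_BP directly, despite a comment describing light damage.
; A duplicate check and debug position prints remain disconnected.
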(event `self.ReceiveActorBeginOverlap`
  (params (OtherActor :type "Actor Object Reference"))
  ;[1 1 1] Check collision type
)

(event `self.Box.OnComponentBeginOverlap`
  (params (OverlappedComponent :type "PrimitiveComponent Object Reference") (OtherActor :type "Actor Object Reference") (OtherComp :type "PrimitiveComponent Object Reference") (OtherBodyIndex :type Integer) (bFromSweep :type Boolean) (SweepResult :type "HitResult Structure (by ref)"))
  (bind _asbp_chaser (cast `/Game/AI/BP_Chaser` (`self.GetOwner`)))
  (bind _returnvalue (`SkeletalMeshComponent.GetAnimInstance` (`Character.Mesh` _asbp_chaser)))
  (bind _returnvalue_2 (`AnimInstance.GetCurrentActiveMontage` _returnvalue))
  (bind _returnvalue_3 (`AnimInstance.Montage_GetPosition` _returnvalue _returnvalue_2))
  (if (and (or (== _returnvalue_2 "/Game/Character/Animation/slash_left_Montage.slash_left_Montage") (== _returnvalue_2 "/Game/Character/Animation/slash_right_Montage.slash_right_Montage")) (== OtherActor (`GameplayStatics.GetPlayerCharacter` 0)) (and (> _returnvalue_3 0.2) (< _returnvalue_3 0.66)))
    ;[1 1 1] Light damage to enemy on hit while attack animation is playing
    (bind _ascharacter_bp (cast `/Game/Character/Character_BP` (`GameplayStatics.GetPlayerCharacter` 0)))
    (`/Game/Character/Character_BP.Event PlayerDeath` _ascharacter_bp)))

(fn `UserConstructionScript`
  (`parent.UserConstructionScript`))