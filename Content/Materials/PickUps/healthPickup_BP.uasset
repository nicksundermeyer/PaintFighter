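; Health pickup Blueprint that heals the player character on overlap and then destroys itself.
; Each Tick offsets the Sphere component vertically by Bounce, while a Delay periodically flips that value's sign to create a bobbing motion.
; The overlap event casts the other actor to Character_BP and calls its Heal function, ignoring any other actor type.
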(event `self.ReceiveTick`
  (params (DeltaSeconds :type "Float (single-precision)"))
  (`SceneComponent.K2_SetWorldLocationAndRotation` :`self` (`self.Sphere`) :`NewLocation` (`KismetMathLibrary.MakeVector` (.x (`SceneComponent.K2_GetComponentLocation` (`self.Sphere`))) (.y (`SceneComponent.K2_GetComponentLocation` (`self.Sphere`))) (+ (.z (`SceneComponent.K2_GetComponentLocation` (`self.Sphere`))) (`self.bounce`))))
  (`KismetSystemLibrary.Delay` 0.1)
  (if (== (`self.bounce`) 0.5)
    (set `self.bounce` -0.5)
    (else
      (set `self.bounce` 0.5))))

(event `self.ReceiveActorBeginOverlap`
  (params (OtherActor :type "Actor Object Reference"))
  (bind _ascharacter_bp (cast `/Game/Character/Character_BP` OtherActor))
  (`/Game/Character/Character_BP.Heal` _ascharacter_bp 1.0)
  (`self.K2_DestroyActor`))

(fn `UserConstructionScript`)