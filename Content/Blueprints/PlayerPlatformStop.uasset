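; A platform actor that moves from its starting position to an end point when the player character steps into its trigger.
; BeginPlay caches the platform's world location and the EndPoint component's location.
; Overlap of the Collision component by a Character_BP plays a timeline that lerps the platform between the two points without sweeping.
; The file contains no reverse or end-overlap logic, so the movement is one-way.
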(event `self.ReceiveBeginPlay`
  (set `self.startLocation` (`SceneComponent.K2_GetComponentLocation` (`self.Platform`)))
  (set `self.endLocation` (`SceneComponent.K2_GetComponentLocation` (`self.EndPoint`))))

(event `self.Collision.OnComponentBeginOverlap`
  (params (OverlappedComponent :type "PrimitiveComponent Object Reference") (OtherActor :type "Actor Object Reference") (OtherComp :type "PrimitiveComponent Object Reference") (OtherBodyIndex :type Integer) (bFromSweep :type Boolean) (SweepResult :type "HitResult Structure (by ref)"))
  (cast `/Game/Character/Character_BP` OtherActor)
  (bind (_direction _newtrack_0) (`Timeline|Timeline_0`)
    (:`Update`
      (`SceneComponent.K2_SetWorldLocation` (`self.Platform`) (`KismetMathLibrary.VLerp` (`self.startLocation`) (`self.endLocation`) _newtrack_0) false false))))

(fn `UserConstructionScript`)