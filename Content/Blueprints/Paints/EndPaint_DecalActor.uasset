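; EndPaint_DecalActor is a paint decal actor that takes on the player character's special color when it spawns.
; On BeginPlay it creates a dynamic material instance on its decal and sets the Color parameter from Character_BP's SpecialColor.
; It copies the character's DecalSortOrder to the decal and increments that shared counter, so each newer decal draws over earlier ones.
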(event `self.ReceiveBeginPlay`
  (bind _decal (`self.Decal`))
  (bind _ascharacter_bp (cast `/Game/Character/Character_BP` (`GameplayStatics.GetPlayerCharacter` 0)))
  (bind _output_get (set `self.Character` _ascharacter_bp))
  (bind _returnvalue (`DecalComponent.CreateDynamicMaterialInstance` _decal))
  (`MaterialInstanceDynamic.SetVectorParameterValue` _returnvalue "Color" (`/Game/Character/Character_BP.SpecialColor` _output_get))
  (bind _decalsortorder (`/Game/Character/Character_BP.DecalSortOrder` _output_get))
  (`DecalComponent.SetSortOrder` _decal _decalsortorder)
  (`/Engine/EditorBlueprintResources/StandardMacros.IncrementInt` _decalsortorder))

(event `self.ReceiveTick`
  (params (DeltaSeconds :type "Float (single-precision)")))

(fn `UserConstructionScript`
  (`parent.UserConstructionScript`))