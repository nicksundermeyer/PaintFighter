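; Distraction actor that, on hit, leaves a paint-like splatter, emits a noise tagged "Distraction" and destroys itself.
; The Splatter function spawns a randomly sized decal at the impact point, oriented along the surface normal.
; It also builds a dynamic material instance with random color and frame, but the decal spawns with the base Splatter_Decal material, leaving that instance unused.
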(event `self.ReceiveHit`
  (params (MyComp :type "PrimitiveComponent Object Reference") (Other :type "Actor Object Reference") (OtherComp :type "PrimitiveComponent Object Reference") (bSelfMoved :type Boolean) (HitLocation :type "Vector Structure") (HitNormal :type "Vector Structure") (NormalImpulse :type "Vector Structure") (Hit :type "HitResult Structure (by ref)"))
  (bind (_bblockinghit _binitialoverlap _time _distance _location _impactpoint _normal) (`GameplayStatics.BreakHitResult` Hit))
  (`self.Splatter` _location _normal)
  (`self.MakeNoise` 1.0 null (0.0 0.0 0.0) 0.0 "Distraction")
  (`self.K2_DestroyActor`))

(fn `Splatter`
  (params (Location :type "Vector Structure") (Normal :type "Vector Structure"))
  (bind _returnvalue (`KismetMathLibrary.RandomFloatInRange` 100.0 150.0))
  (bind _returnvalue_2 (`KismetMaterialLibrary.CreateDynamicMaterialInstance` "/Game/Materials/Splatter_Decal.Splatter_Decal"))
  (`MaterialInstanceDynamic.SetVectorParameterValue` _returnvalue_2 "Color" (`KismetMathLibrary.MakeColor` (`KismetMathLibrary.RandomFloatInRange` 0.0 1.0) (`KismetMathLibrary.RandomFloatInRange` 0.0 1.0) (`KismetMathLibrary.RandomFloatInRange` 0.0 1.0)))
  (`MaterialInstanceDynamic.SetScalarParameterValue` _returnvalue_2 "Frame" (`KismetMathLibrary.Conv_IntToDouble` (`KismetMathLibrary.RandomInteger` 15)))
  (`GameplayStatics.SpawnDecalAtLocation` "/Game/Materials/Splatter_Decal.Splatter_Decal" (`KismetMathLibrary.MakeVector` _returnvalue _returnvalue _returnvalue) Location (`KismetMathLibrary.Conv_VectorToRotator` Normal)))

(fn `UserConstructionScript`)