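; Heavy attack actor that damages BP_Chaser pawns and sprays splatter decals.
; On BeginPlay it activates its particle system and runs a one-time Box overlap query, calling TakeHeavyDamage on each Chaser found and destroying the Box.
; Particle collisions spawn randomly sized decals aligned to the hit normal.
; A random color and frame are set on a dynamic material instance, but the decal spawns with the base Splatter_Decal material.
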(event `self.ReceiveBeginPlay`
  (bind _particlesystem (`self.ParticleSystem`))
  (bind _box (`self.Box`))
  ;[1 1 1] Playing particle system and adding splatter based on collisions
  (`ActorComponent.Activate` _particlesystem false)
  (add `ParticleSystemComponent.OnParticleCollide` _particlesystem (delegate `Splatter Collision`))
  ;[1 1 1] Checking for collided actors to damage them
  (bind _outactors (`KismetSystemLibrary.ComponentOverlapActors` _box (`SceneComponent.K2_GetComponentToWorld` _box) (`|MakeArray` "ObjectTypeQuery3" :!type "EObjectTypeQuery Enum") "/Game/AI/BP_Chaser.BP_Chaser_C"))
  (for _array_element _outactors
    (bind _asbp_chaser (cast `/Game/AI/BP_Chaser` _array_element))
    (`/Game/AI/BP_Chaser.TakeHeavyDamage` _asbp_chaser)
    (`ActorComponent.K2_DestroyComponent` (`self.Box`))))

(event `Splatter Collision`
  (params (EventName :type Name) (EmitterTime :type "Float (double-precision)") (ParticleTime :type Integer) (Location :type "Vector Structure") (Velocity :type "Vector Structure") (Direction :type "Vector Structure") (Normal :type "Vector Structure") (BoneName :type Name) (PhysMat :type "PhysicalMaterial Object Reference"))
  ;[1 1 1] Playing particle system and adding splatter based on collisions
  (bind _returnvalue (`KismetMaterialLibrary.CreateDynamicMaterialInstance` "/Game/Materials/Splatter_Decal.Splatter_Decal"))
  (`MaterialInstanceDynamic.SetVectorParameterValue` _returnvalue "Color" (`KismetMathLibrary.MakeColor` (`KismetMathLibrary.RandomFloatInRange` 0.0 1.0) (`KismetMathLibrary.RandomFloatInRange` 0.0 1.0) (`KismetMathLibrary.RandomFloatInRange` 0.0 1.0)))
  (`MaterialInstanceDynamic.SetScalarParameterValue` _returnvalue "Frame" (`KismetMathLibrary.Conv_IntToDouble` (`KismetMathLibrary.RandomInteger` 15)))
  (`GameplayStatics.SpawnDecalAtLocation` "/Game/Materials/Splatter_Decal.Splatter_Decal" (`KismetMathLibrary.Conv_DoubleToVector` (`KismetMathLibrary.RandomFloatInRange` 20.0 50.0)) Location (`KismetMathLibrary.Conv_VectorToRotator` Normal)))

(event `self.ReceiveActorBeginOverlap`
  (params (OtherActor :type "Actor Object Reference")))

(fn `UserConstructionScript`)