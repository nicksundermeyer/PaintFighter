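; EndLevel is a level-exit actor that reacts to any actor overlap by resetting the game instance's saved checkpoint location.
; It opens the level named by NextLevel unless that name is "GameOver".
; The GameOver branch only creates a dynamic mural decal material and casts the player character.
; The pickup-based mural dissolve, ending-camera blend and end screen (noted as not working) are disconnected and never run.
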(event `self.ReceiveActorBeginOverlap`
  (params (OtherActor :type "Actor Object Reference"))
  (bind _asbp_blank_canvas_game_instance (cast `/Game/Blueprints/BP_BlankCanvasGameInstance` (`GameplayStatics.GetGameInstance`)))
  (set `/Game/Blueprints/BP_BlankCanvasGameInstance.LatestCheckpointLoc` (0.0 0.0 0.0) _asbp_blank_canvas_game_instance)
  (if (`KismetStringLibrary.NotEqual_StrStr` (`KismetStringLibrary.Conv_NameToString` (`self.NextLevel`)) "GameOver")
    (`GameplayStatics.OpenLevel` (`self.NextLevel`))
    (else
      ;[1 1 1] Creating mural decal
      (bind _returnvalue (`KismetMaterialLibrary.CreateDynamicMaterialInstance` "/Game/Materials/Mural_Decal.Mural_Decal"))
      (bind _ascharacter_bp (cast `/Game/Character/Character_BP` (`GameplayStatics.GetPlayerCharacter` 0))))))

(fn `UserConstructionScript`)